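; Stealth enemy character that patrols random points or a target-point loop, chases a seen player, and investigates noises.
; Tick picks patrol or chase via CanMove, CanChase and PlayerVisible flags, with AIMoveTo handling movement.
; PawnSensing drives detection, and a looping timer clears sight after a timeout.
; Reaching the player triggers a montage attack whose notify sphere-traces from the hand and reloads the hit player's checkpoint; rock-distraction logic is unwired.
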(event OnHearNoise(PawnSensing)
  (params (Instigator :type Pawn%20Object%20Reference) (Location :type Vector%20%28by%20ref%29 :default "0, 0, 0") (Volume :type Float%20%28single-precision%29))
  ;[0.15 0.15 0.15 0.5] Can AI Hear Player
  (Development|PrintString "Hello")
  (if (not (Variables|Default|GetbPlayerVisible))
    (Development|PrintString "WHAT WAS THAT SOUND?")
    (CallFunction|UpdateWalkSpeed 0.0)
    (Variables|Default|SetbCanMove false)
    (AI|AIMoveTo self Location Instigator 5.0 false
      (:OnSuccess
        (Utilities|FlowControl|Delay 2e+01)
        (Variables|Default|SetbCanMove true)))))

(event OnSeePawn(PawnSensing)
  (params (Pawn :type Pawn%20Object%20Reference))
  ;[0.15 0.15 0.15 0.5] When Ai sees player
  (if (Actor|ActorHasTag Pawn "Player")
    (Development|PrintString "I SEE YOU!")
    (Variables|Default|SetbPlayerVisible true)
    (Variables|Default|SetLastSeenTime (Utilities|Time|GetTimeSeconds))
    (bind _returnvalue (Utilities|Time|SetTimerbyFunctionName 0 "CheckLostSight" 0.5 true true))
    (Variables|Default|SetCheckLastSightHandler _returnvalue)))

(event Custom|ChasePlayer
  ;[0.15 0.15 0.15 0.5] AI Chases Player
  (CallFunction|UpdateWalkSpeed 4e+02)
  (Variables|Default|SetbCanMove false)
  (Variables|Default|SetbCanChase false)
  (AI|AIMoveTo self "0, 0, 0" (Game|GetPlayerCharacter 0) 5.0 false
    (:OnSuccess
      (CallFunction|Attack))
    (:OnFail
      _))
  (Utilities|FlowControl|Delay 2.0)
  (Variables|Default|SetbCanMove true)
  (Variables|Default|SetbCanChase true))

(event Custom|Attack
  (bind _mesh (Variables|Character|GetMesh))
  (bind _returnvalue (Transformation|GetSocketLocation _mesh "hand_r"))
  ;[0.15 0.15 0.15 0.5] Melee Attack
  (Utilities|FlowControl|DoOnce false
    (:Completed
      (bind _notifyname (Animation|Montage|PlayMontage (Variables|Character|GetMesh) "/Game/StealthGame/Characters/Enemies/AM_Attack_01.AM_Attack_01")
        (:OnCompleted
          (CallFunction|ResetAttack))
        (:OnNotifyBegin
          (switch name _notifyname
            (:AttackDamage
              (Development|PrintString "IM ATTACKING")
              (bind (_outhits _returnvalue_2) (Collision|MultiSphereTraceForObjects _returnvalue (+ _returnvalue (* (Transformation|GetActorForwardVector) (Variables|Default|GetMeleeTraceDistance))) (Variables|Default|GetMeleeTraceRadius) (Utilities|Array|MakeArray "ObjectTypeQuery3") false 0 "ForOneFrame"))
              (if _returnvalue_2
                (for _array_element _outhits
                  (bind _asbp_third_person_character_custom (Utilities|Casting|CastToBP_ThirdPersonCharacterCustom (.HitActor (Collision|BreakHitResult _array_element))))
                  (Default|LoadCheckpoint _asbp_third_person_character_custom))))))))))

(event Custom|PatrolTargets
  ;[0.15 0.15 0.15 0.5] Patrol Random Targets
  (CallFunction|MovetoNextTargetPoint))

(event Custom|ResetAttack
  (bind _mesh (Variables|Character|GetMesh))
  (bind _returnvalue (Transformation|GetSocketLocation _mesh "hand_r"))
  ;[0.15 0.15 0.15 0.5] Melee Attack
  (Utilities|FlowControl|DoOnce false) ; enters at Reset
)

(event Custom|MoveToNextTargetPoint
  ;[0.15 0.15 0.15 0.5] AI Patrols to next target point
  (CallFunction|UpdateWalkSpeed 2e+02)
  (Variables|Default|SetbCanMove false)
  (AI|AIMoveTo self "0, 0, 0" (Utilities|Array|Get(acopy) (Variables|Default|GetPatrolTargetPoints) (Variables|Default|GetCurrentIndex)) 3e+01 false
    (:OnSuccess
      (Utilities|FlowControl|Delay 4.0)
      (CallFunction|GetNextPatrolPoint)
      (Variables|Default|SetbCanMove true))))

(event Custom|CheckLostSight
  ;[0.15 0.15 0.15 0.5] AI Looks for player in eye-sight
  (if (> (- (Utilities|Time|GetTimeSeconds) (Variables|Default|GetLastSeenTime)) (Variables|Default|GetSightTimeout))
    (Variables|Default|SetbPlayerVisible false)
    (Utilities|Time|ClearandInvalidateTimerbyHandle (Variables|Default|GetCheckLastSightHandler))
    (Development|PrintString "Target Lost")))

(event Custom|RandomPatrol
  ;[0.15 0.15 0.15 0.5] Patrol
  (CallFunction|UpdateWalkSpeed 2e+02)
  (Variables|Default|SetbCanMove false)
  (AI|AIMoveTo self (.RandomLocation (AI|Navigation|GetRandomReachablePointinRadius (Transformation|GetActorLocation) 2e+03 0 0)) 0 15.0 false
    (:OnSuccess
      (Utilities|FlowControl|Delay 2.0)
      (Variables|Default|SetbCanMove true))))

(event Custom|GetNextPatrolPoint
  ;[0.15 0.15 0.15 0.5] Patrol Random Targets
  (Variables|Default|SetCurrentIndex (Math|Integer|%(Integer) (+ (Variables|Default|GetCurrentIndex) 1) (Utilities|Array|Length (Variables|Default|GetPatrolTargetPoints)))))

(event EventTick
  (params (DeltaSeconds :type Float%20%28single-precision%29))
  ;[0.15 0.15 0.15 0.5] Event Tick
  (if (Variables|Default|GetbCanMove)
    (if (Variables|Default|GetbPlayerVisible)
      (CallFunction|ChasePlayer)
      (else
        (switch Utilities|FlowControl|Switch|SwitchonBPE_PatrolType (Variables|Default|GetPatrolType)
          (:NewEnumerator0
            (CallFunction|RandomPatrol))
          (:NewEnumerator1
            (CallFunction|PatrolTargets)))))
    (elif (and (Variables|Default|GetbPlayerVisible) (Variables|Default|GetbCanChase))
      (Components|Movement|StopMovementImmediately (Variables|Character|GetCharacterMovement))
      (CallFunction|ChasePlayer))))

(fn ConstructionScript)

(fn UpdateWalkSpeed
  (params (NewWalkSpeed :type Float%20%28double-precision%29))
  (Variables|/Script/Engine.CharacterMovementComponent|SetMaxWalkSpeed (Variables|Character|GetCharacterMovement) NewWalkSpeed))