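; BP_RockDistraction is a rock that creates a noise distraction for AI in the stealth game.
; On its first hit against anything other than the player, it plays the rock sound and reports a loud, range-limited AI noise event at its location.
; The noise names the player as instigator, and a DoOnce keeps later hits silent.
; Leftover pawn noise emitter and stimuli source nodes are unconnected and never run.
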(event Collision|EventHit
  (params (MyComp :type Primitive%20Component%20Object%20Reference) (Other :type Actor%20Object%20Reference) (OtherComp :type Primitive%20Component%20Object%20Reference) (bSelfMoved :type Boolean) (HitLocation :type Vector :default "0, 0, 0") (HitNormal :type Vector :default "0, 0, 0") (NormalImpulse :type Vector :default "0, 0, 0") (Hit :type Hit%20Result%20Structure%20%28by%20ref%29))
  (bind _returnvalue (Game|GetPlayerCharacter 0))
  (bind _returnvalue_2 (Transformation|GetActorLocation))
  (if (!= Other _returnvalue)
    (Utilities|FlowControl|DoOnce false
      (:Completed
        (Audio|PlaySoundatLocation "/Game/StealthGame/Sound/RockAudioCue.RockAudioCue" _returnvalue_2 "0, 0, 0" 1.0 1.0 0.0 0 0 0 0)
        (Class|AISenseHearing|ReportNoiseEvent _returnvalue_2 1e+02 _returnvalue 3e+03 "None")))))

(fn ConstructionScript)