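; BP_Clown is an AI-moved clown that walks on stage, turns toward the audience for its joke beat, then heads to a destination.
; BeginPlay starts the AI move to its walk point, and success triggers TellJoke, which currently only prints debug text.
; GetPunched enables physics, launches the clown along the camera's forward vector with added lift, and has the manager spawn another clown after a delay.
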(event Custom|Tell%20Joke
  (Transformation|SetActorRotation (Math|Rotator|MakeRotator 0.0 0.0 (.yaw (Math|Interpolation|RInterpTo (Transformation|GetActorRotation) (Math|Rotator|MakeRotator 0.0 0.0 (.yaw (Math|Rotator|FindLookatRotation (Transformation|GetActorLocation) (Transformation|GetActorLocation (Variables|Default|GetTheAudience))))) (Utilities|Time|GetWorldDeltaSeconds) 5e+02))))
  (Development|PrintString "Yes")
  (Utilities|FlowControl|Delay 3.0)
  (AI|AIMoveTo self "0, 0, 0" (Variables|Default|GetDestination) 5.0 false
    (:then
      (Development|PrintString "Uh huh"))
    (:OnSuccess
      (Development|PrintString "And we succeeded"))
    (:OnFail
      (Development|PrintString "Ditto"))))

(event Custom|Walk%20On%20Stage
  (if (not (Variables|Default|GetbMadeit))
    (Development|PrintString (Utilities|GetObjectName (Variables|Default|GetClownWalkPoint)))
    (AI|AIMoveTo self "0, 0, 0" (Variables|Default|GetClownWalkPoint) 5e+01 false
      (:OnSuccess
        (Variables|Default|SetbMadeit true)
        (CallFunction|TellJoke)
        (Development|PrintString "Mewtwo"))
      (:OnFail
        (Development|PrintString "Hello")))))

(event Custom|Get%20Punched
  (bind _mesh (Variables|Character|GetMesh))
  (bind _camera (Variables|Default|GetCamera))
  (bind _returnvalue (Transformation|GetWorldRotation _camera))
  (bind _returnvalue_2 (Math|Vector|GetForwardVector _returnvalue))
  (bind _returnvalue_3 (* _returnvalue_2 5e+03))
  (Physics|SetSimulatePhysics _mesh true)
  (Physics|AddImpulse _mesh (Math|Vector|MakeVector (.x _returnvalue_3) (.y _returnvalue_3) (+ (.z _returnvalue_3) 1e+03)) "None" true)
  (Variables|Default|SetbNoMoreClown true)
  (CallFunction|MakeMore)
  (Variables|Default|SetbMadeit true))

(event Custom|MakeMore
  (if (Variables|Default|GetbNoMoreClown)
    (Utilities|FlowControl|Delay 3.0)
    (Default|SpawnClown (Variables|Default|GetManager))))

(event EventBeginPlay
  (CallFunction|WalkonStage))

(event Collision|EventActorBeginOverlap
  (params (OtherActor :type Actor%20Object%20Reference)))

(event EventTick
  (params (DeltaSeconds :type Float%20%28single-precision%29)))

(fn ConstructionScript)