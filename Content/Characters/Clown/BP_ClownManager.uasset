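; BP_ClownManager supplies clowns with their shared stage references and spawns new ones to walk on stage.
; On BeginPlay it gathers every placed BP_Clown and assigns itself, the walk point, audience target and leaving destination.
; SpawnClown creates a clown at the spawn point, sets the manager and walk point, waits briefly, then assigns audience and destination before calling WalkOnStage.
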(event Custom|SpawnClown
  (bind _returnvalue (Game|SpawnActorfromClass "/Game/Characters/Clown/BP_Clown.BP_Clown_C" (Transformation|GetActorTransform (Variables|Default|GetClownSpawnPoint)) "Undefined" "MultiplyWithRoot" 0 0))
  (Variables|/Game/Characters/Clown/BP_Clown.BP_Clown_C|SetManager _returnvalue self)
  (Variables|/Game/Characters/Clown/BP_Clown.BP_Clown_C|SetClownWalkPoint _returnvalue (Variables|Default|GetClownDirectPoint))
  (Utilities|FlowControl|Delay 0.2)
  (Variables|/Game/Characters/Clown/BP_Clown.BP_Clown_C|SetTheAudience _returnvalue (Variables|Default|GetClownTarget))
  (Variables|/Game/Characters/Clown/BP_Clown.BP_Clown_C|SetDestination _returnvalue (Variables|Default|GetClownLeavingPoint))
  (Default|WalkonStage _returnvalue))

(event Custom|Set%20Manager
  (for _array_element (Variables|Default|GetClowns)
    (Variables|/Game/Characters/Clown/BP_Clown.BP_Clown_C|SetManager _array_element self)
    (Variables|/Game/Characters/Clown/BP_Clown.BP_Clown_C|SetClownWalkPoint _array_element (Variables|Default|GetClownDirectPoint))
    (Variables|/Game/Characters/Clown/BP_Clown.BP_Clown_C|SetTheAudience _array_element (Variables|Default|GetClownTarget))
    (Variables|/Game/Characters/Clown/BP_Clown.BP_Clown_C|SetDestination _array_element (Variables|Default|GetClownLeavingPoint))))

(event EventBeginPlay
  (bind _outactors (Actor|GetAllActorsOfClass "/Game/Characters/Clown/BP_Clown.BP_Clown_C"))
  (Variables|Default|SetClowns _outactors)
  (CallFunction|SetManager))

(event Collision|EventActorBeginOverlap
  (params (OtherActor :type Actor%20Object%20Reference)))

(event EventTick
  (params (DeltaSeconds :type Float%20%28single-precision%29)))

(fn ConstructionScript)